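; BPFL_Utilities is a Blueprint function library of small, independent helpers.
; GetHitResult runs a complex trace under the first player's cursor on the Visibility channel.
; GetForwardAndRightVectors derives both direction vectors from a rotation.
; CalculateVelocity converts an actor's world velocity into its local space using an inverse transform direction.
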(fn GetHitResult
  (return (.HitResult (Game|Player|GetHitResultUnderCursorbyChannel (Game|GetPlayerController 0) "TraceTypeQuery1" true))))

(fn GetForwardandRightVectors
  (params (InRot :type Rotator))
  (return (Math|Vector|GetForwardVector InRot) (Math|Vector|GetRightVector InRot)))

(fn CalculateVelocity
  (params (Actor :type Actor%20Object%20Reference))
  (return (Math|Transform|InverseTransformDirection (Transformation|GetActorTransform Actor) (Transformation|GetVelocity Actor))))
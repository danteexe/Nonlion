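; Player ability component that implements a dash, caching the player character and its skeletal mesh through interface messages on BeginPlay.
; DashAbility runs only when the character is idle, sets it to Dashing, plays a montage and restores Idle when the montage completes.
; It launches the character along its last movement input, or capsule forward without input, with fixed lift.
; A DoOnce and Delay enforce the cooldown, shown by a widget animation.
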(event Custom|DashAbility
  (bind _characterref (Variables|References|GetCharacterRef))
  (bind (_returnvalue_x _returnvalue_y) (CallFunction|GetLaunchVelocity _characterref))
  ;[0.02499 0.05098 0.05729 1 50] Dash
  (bind _condition (Class|BPICharacter|IsPlayerIdle(Message) (Variables|References|GetCharacterRef)))
  (if _condition
    (Utilities|FlowControl|DoOnce false :!label _label
      (:Completed
        (Class|BPICharacter|SetPlayerCondition(Message) (Variables|References|GetCharacterRef) "NewEnumerator1")
        (Animation|Montage|PlayMontage (Variables|References|GetSKRef) (Variables|AbilityDash|GetDash%20Animation)
          (:then
            (Character|LaunchCharacter _characterref (Math|Vector|MakeVector _returnvalue_x _returnvalue_y 3e+02) false false)
            (CallFunction|PlayDashAnimation)
            (Utilities|FlowControl|Delay (Variables|AbilityDash|GetDash%20Cooldown))
            (goto _label Reset))
          (:OnCompleted
            (Class|BPICharacter|SetPlayerCondition(Message) (Variables|References|GetCharacterRef) "NewEnumerator0")))))))

(event EventBeginPlay
  ;[1 1 1 1 50] Evet BeginPlay
  (bind _getself (Class|BPICharacter|CastCharacter(Message) (Game|GetPlayerCharacter 0)))
  (bind _output_get (Variables|References|SetCharacterRef _getself))
  (bind _skref (Class|BPICharacter|GetSkeletalMeshComponent(Message) _output_get))
  (Variables|References|SetSKRef _skref))

(event EventTick
  (params (DeltaSeconds :type Float%20%28single-precision%29)))

(fn GetLaunchVelocity
  (params (Target :type Character%20Object%20Reference))
  (bind _returnvalue (CallFunction|SelectDashLocation Target))
  (bind _dash_power (Variables|AbilityDash|GetDash%20Power))
  (bind _returnvalue_2 (Math|Vector|Normalize _returnvalue))
  (bind _returnvalue_3 (* _returnvalue_2 _dash_power))
  (return (.x _returnvalue_3) (.y _returnvalue_3)))

(fn SelectDashLocation
  (params (Target :type Character%20Object%20Reference))
  (bind _returnvalue (Class|Pawn|GetLastMovementInputVector Target))
  (if (Class|KismetMathLibrary|EqualExactlyVectorVector _returnvalue "0, 0, 0")
    (return (Math|Vector|GetForwardVector (Variables|/Script/Engine.Character|GetCapsuleComponent Target)))
    (else
      (return _returnvalue))))

(fn IsPlayerIdle
  (bind _condition (Class|BPICharacter|GetPlayerCondition(Message) (Variables|References|GetCharacterRef)))
  (switch Utilities|FlowControl|Switch|SwitchonE_PlayerCondition _condition
    (:NewEnumerator0
      (return true))
    (:NewEnumerator1
      _)
    (:NewEnumerator2
      _))
  (return false))

(fn PlayDashAnimation
  (bind _widget (Class|BPICharacter|GetDashWidget(Message) (Variables|References|GetCharacterRef)))
  (Class|UserWidget|PlayAnimationForward _widget (Variables|/Game/_Core/Blueprints/Widget/WBP_DashAbility.WBP_DashAbility_C|GetDashCoolDown _widget) 1.0 false))